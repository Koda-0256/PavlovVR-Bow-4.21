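; BP_ItemSpawner is a Pavlov VR pickup point that spawns a bow or arrow into the interacting player's hand.
; Mesh interactions replicate to the server through the hand proxy; bows respond to grab, other items to trigger.
; The server spawns the ItemMap class at the hand resolved from dominance and handedness, then calls GrabBow or GrabArrow.
; The construction script sets the display mesh from the same map entry.
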(event `self.Mesh.OnInteractSMClient`
  (params (InteractType :type "EInteractType Enum" :default "Grabbed") (HandProxy :type "Pavlov_HandProxy Object Reference") (InteractMesh :type "Pavlov_InteractStaticMesh Object Reference"))
  (`Pavlov_HandProxy.ReplicateInteract_Server` HandProxy InteractType InteractMesh))

(event `self.Mesh.OnInteractSMServer`
  (params (InteractType :type "EInteractType Enum" :default "Grabbed") (HandProxy :type "Pavlov_HandProxy Object Reference") (InteractMesh :type "Pavlov_InteractStaticMesh Object Reference"))
  (bind _bdominanthand (`Pavlov_HandProxy.bDominantHand` HandProxy))
  (bind (_value _returnvalue) (`BlueprintMapLibrary.Map_Find` (`self.Item Map`) (`self.Item`)))
  (bind _returnvalue_2 (select `/Game/Blueprints/Items/ECustomItemList` (`self.Item`) :`NewEnumerator0` true))
  (switch `EInteractType` InteractType
    (:`Grabbed`
      (if _returnvalue_2
        (bind _playerstatus (`PavlovProxyStatics.GetPavlovPlayerStatusByPawn` (`Pavlov_PlayerProxy.GetPawn` (`Pavlov_HandProxy.GetPlayerProxy` HandProxy)) :!label _label))
        (bind (_successful_ _left_hand _right_hand) (`/CustomMapTools/Blueprints/BPFL_PavlovTemplate.GetHands` (`.Pawn` (break `PavlovPlayerStatus` _playerstatus))))
        (if _returnvalue
          (bind _returnvalue_3 (select `bool` (`.bRightHanded` (break `PavlovPlayerStatus` _playerstatus)) :`false` (not _bdominanthand) :`true` _bdominanthand))
          (bind _returnvalue_4 (select `bool` _returnvalue_3 :`false` _left_hand :`true` _right_hand))
          (bind _returnvalue_5 (`|SpawnActorFromClass` (break `/Game/Blueprints/Items/CustomItemStruct` _value) (`SceneComponent.K2_GetComponentToWorld` _returnvalue_4) "Undefined" "OverrideRootScale" null null))
          (bind _asbow_base (cast `/Game/Blueprints/Items/Bow/Bow_Base` _returnvalue_5)
            (:`then`
              (bind _returnvalue_6 (not _returnvalue_3))
              (`/Game/Blueprints/Items/Bow/Bow_Base.Grab Bow` _asbow_base (`.Pawn` (break `PavlovPlayerStatus` _playerstatus)) _returnvalue_4 _returnvalue_6))
            (:`CastFailed`
              (bind _asarrow_base (cast `/Game/Blueprints/Items/Bow/Arrow_Base` _returnvalue_5))
              (`/Game/Blueprints/Items/Bow/Arrow_Base.Grab Arrow` _asarrow_base (`.Pawn` (break `PavlovPlayerStatus` _playerstatus)) _returnvalue_4 _returnvalue_6))))))
    (:`Trigger`
      (if (not _returnvalue_2)
        (goto _label)))))

(fn `UserConstructionScript`
  (bind _mesh (`self.Mesh`))
  (bind (_value _returnvalue) (`BlueprintMapLibrary.Map_Find` (`self.Item Map`) (`self.Item`)))
  (if _returnvalue
    (`StaticMeshComponent.SetStaticMesh` _mesh (`.Mesh_6_04C9166C4112F1B5E5D28A87EBA9E0F3` (break `/Game/Blueprints/Items/CustomItemStruct` _value)))
    (else
      (`StaticMeshComponent.SetStaticMesh` _mesh null))))