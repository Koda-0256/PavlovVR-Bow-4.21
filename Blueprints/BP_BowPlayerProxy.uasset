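; Per-player proxy for a Pavlov VR bow mod that relays bow, arrow and quiver interactions for its pawn.
; Grabs drop any native item held in that hand, mapping left/right to dominant hand through the player's handedness.
; It spawns quivers that OnRep attaches to the spine, saves arrow counts to the bow on removal, and destroys them on death.
; GivePlayerItem spawns a bow or arrow directly into a chosen hand.
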(event `Server Override Pickup`
  (params (`Left Hand` :type Boolean))
  (`KismetSystemLibrary.Delay` 0.1)
  (`self.Override Pickup` `Left Hand`))

(event `Replicate Interact Arrow`
  (params (Arrow :type "/Game/Blueprints/Items/Bow/Arrow_Base Object Reference") (`Motion Controller` :type "MotionControllerComponent Object Reference") (`Left Hand` :type Boolean))
  (`/Game/Blueprints/Items/Bow/Arrow_Base.Grab Arrow` Arrow (`self.GetPawn`) `Motion Controller` `Left Hand`)
  (`/Engine/EditorBlueprintResources/StandardMacros.IsValid` `Motion Controller`
    (:`Is Valid`
      (`self.Override Pickup` `Left Hand`))))

(event `Replicate Interact Bow`
  (params (String :type Boolean) (Bow :type "/Game/Blueprints/Items/Bow/Bow_Base Object Reference") (`Motion Controller` :type "MotionControllerComponent Object Reference") (`Left Hand` :type Boolean))
  (if String
    (`/Game/Blueprints/Items/Bow/Bow_Base.Grab String` Bow `Motion Controller`)
    (else
      (`/Game/Blueprints/Items/Bow/Bow_Base.Grab Bow` Bow (`self.GetPawn`) `Motion Controller` `Left Hand`)))
  (`/Engine/EditorBlueprintResources/StandardMacros.IsValid` `Motion Controller`
    (:`Is Valid`
      (`self.Override Pickup` `Left Hand`))))

(event `self.OnPlayerDeath`
  (params (KilledActor :type "Actor Object Reference"))
  (bind _quiver (`self.Quiver`))
  (`/Engine/EditorBlueprintResources/ActorMacros.Switch Has Authority`
    (:`Authority`
      (`self.Player Death`)
      (`/Engine/EditorBlueprintResources/StandardMacros.IsValid` _quiver
        (:`Is Valid`
          (`self.K2_DestroyActor` _quiver))))))

(event `Spawn Quiver`
  (params (Bow :type "/Game/Blueprints/Items/Bow/Bow_Base Object Reference") (`Quiver Class` :type "/Game/Blueprints/Items/Bow/Quiver_Base Class Reference") (Arrows :type "Array of /Game/Blueprints/Items/Bow/Arrow_Base Class Reference"))
  (bind _quiver (`self.Quiver`))
  (`/Engine/EditorBlueprintResources/StandardMacros.IsValid` _quiver
    (:`Is Valid`
      (`self.K2_DestroyActor` _quiver))
    (:`Is Not Valid`
      _))
  (bind _returnvalue (`|SpawnActorFromClass` `Quiver Class` (`KismetMathLibrary.MakeTransform` (0.0 0.0 0.0)) "Undefined" "OverrideRootScale" (`Pawn.PlayerState` (`self.GetPawn`)) false 18 Bow Arrows null))
  (set `self.Quiver` _returnvalue))

(event `Remove Quiver`
  (params (Bow :type "/Game/Blueprints/Items/Bow/Bow_Base Object Reference"))
  (bind _quiver (`self.Quiver`))
  (`/Engine/EditorBlueprintResources/StandardMacros.IsValid` _quiver
    (:`Is Valid`
      (set `/Game/Blueprints/Items/Bow/Bow_Base.Stored Arrows` (`/Game/Blueprints/Items/Bow/Quiver_Base.Arrows` _quiver) Bow)
      (`self.K2_DestroyActor` _quiver))))

(event `Replicate Interact Quiver`
  (params (Quiver :type "/Game/Blueprints/Items/Bow/Quiver_Base Object Reference") (`Motion Controller` :type "MotionControllerComponent Object Reference") (`Left Hand` :type Boolean))
  (`/Game/Blueprints/Items/Bow/Quiver_Base.Interact Quiver` Quiver (`self.GetPawn`) `Motion Controller` `Left Hand`))

(fn `Give Player Item`
  (params (Class :type "Actor Object Reference") (`Dominant Hand` :type Boolean))
  (returns (Successful :type Boolean) (Item :type "Actor Object Reference"))
  (bind _returnvalue (`self.GetPawn`))
  (`/Engine/EditorBlueprintResources/StandardMacros.IsValid` _returnvalue
    (:`Is Valid`
      (bind _playerstatus (`PavlovProxyStatics.GetPavlovPlayerStatusByPawn` _returnvalue))
      (bind (_successful_ _left_hand _right_hand) (`/CustomMapTools/Blueprints/BPFL_PavlovTemplate.GetHands` _returnvalue))
      (bind _returnvalue_2 (select `bool` (`.bRightHanded` (break `PavlovPlayerStatus` _playerstatus)) :`false` (not `Dominant Hand`) :`true` `Dominant Hand`))
      (bind _returnvalue_3 (select `bool` _returnvalue_2 :`false` _left_hand :`true` _right_hand))
      (bind _returnvalue_4 (`|SpawnActorFromClass` Class (`SceneComponent.K2_GetComponentToWorld` _returnvalue_3) "Undefined" "OverrideRootScale" null null))
      (bind _asbow_base (cast `/Game/Blueprints/Items/Bow/Bow_Base` _returnvalue_4)
        (:`then`
          (bind _returnvalue_5 (not _returnvalue_2))
          (`/Game/Blueprints/Items/Bow/Bow_Base.Grab Bow` _asbow_base _returnvalue _returnvalue_3 _returnvalue_5)
          (return true _asbow_base))
        (:`CastFailed`
          (bind _asarrow_base (cast `/Game/Blueprints/Items/Bow/Arrow_Base` _returnvalue_4))
          (`/Game/Blueprints/Items/Bow/Arrow_Base.Grab Arrow` _asarrow_base _returnvalue _returnvalue_3 _returnvalue_5)
          (return true _asarrow_base))))
    (:`Is Not Valid`
      (return false null))))

(fn `OnRep_Overriden Item`
  (bind _overridden_item (`self.Overridden Item`))
  (`/Engine/EditorBlueprintResources/StandardMacros.IsValid` _overridden_item
    (:`Is Valid`
      (`SceneComponent.SetHiddenInGame` (`self.K2_GetComponentsByClass` _overridden_item "/Script/Engine.SceneComponent") false false))))

(fn `OnRep_Quiver`
  (bind _quiver (`self.Quiver`))
  (`/Engine/EditorBlueprintResources/StandardMacros.IsValid` _quiver
    (:`Is Valid`
      (`SceneComponent.K2_AttachToComponent` (`/Game/Blueprints/Items/Bow/Quiver_Base.Quiver Root` _quiver) (`self.GetPlayerSkeleton`) "Spine_02" "SnapToTarget" "SnapToTarget" "KeepWorld" true))))

(fn `Override Pickup`
  (params (`Left Hand` :type Boolean))
  (set `self.Overridden Item` null)
  (bind _playerstatus (`PavlovProxyStatics.GetPavlovPlayerStatusByPawn` (`self.GetPawn`)))
  (bind _returnvalue (select `bool` (`.bRightHanded` (break `PavlovPlayerStatus` _playerstatus)) :`false` `Left Hand` :`true` (not `Left Hand`)))
  (bind (_bhasitem _item) (`self.GetHeldItem` _returnvalue))
  (if _bhasitem
    (set `self.Overridden Item` (break `PlayerItem` _item))
    (`self.DropHeld` (select `bool` _returnvalue :`false` "NonDominant" :`true` "Dominant" :!type "EHands Enum")))
  (return))

(fn `UserConstructionScript`)